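; Player controller that handles swapping between Skvt characters and toggling a pausing main menu.
; On BeginPlay it adds the default, pawn-swap and camera Enhanced Input mapping contexts.
; Swap input gathers all BP_SkvtBaseChar actors and possesses the one after the controlled pawn, wrapping to the first.
; Menu input creates or removes WBP_MainMenu, using the widget reference as open state, and switches cursor, input mode and pause.
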(event Input|EnhancedActionEvents|EnhancedInputActionIA_Swap
  (params (ActionValue :type Boolean) (ElapsedSeconds :type Float%20%28double-precision%29) (TriggeredSeconds :type Float%20%28double-precision%29) (InputAction :type Input%20Action%20Object%20Reference :default "/Game/Skvt/Characters/Input/Actions/IA_Swap.IA_Swap"))
  ;[0.1667 0.1667 0.1667] Swap character script (reworked)
  (bind _outactors (Actor|GetAllActorsOfClass "/Game/Skvt/Characters/BP_SkvtBaseChar.BP_SkvtBaseChar_C"))
  (Pawn|Possess (CallFunction|FindNextChar _outactors)))

(event Input|EnhancedActionEvents|EnhancedInputActionIA_OpenMenu
  (params (ActionValue :type Boolean) (ElapsedSeconds :type Float%20%28double-precision%29) (TriggeredSeconds :type Float%20%28double-precision%29) (InputAction :type Input%20Action%20Object%20Reference :default "/Game/Skvt/Characters/Input/Actions/IA_OpenMenu.IA_OpenMenu"))
  ;[0.2448 0.2448 0.2448] Open menu mechanic
  (if (CallFunction|IsMenuOpen)
    (CallFunction|CloseMenu)
    (else
      (CallFunction|OpenMenu))))

(event EventBeginPlay
  (bind _self self)
  (bind _returnvalue (PlayerController|LocalPlayerSubsystems|GetEnhancedInputLocalPlayerSubsystem _self))
  ;[0.1562 0.1562 0.1562] Mapping Contexts
  (Utilities|IsValid _returnvalue
    (:Is%20Valid
      (Input|AddMappingContext _returnvalue "/Game/ThirdPerson/Input/IMC_Default.IMC_Default" 0 "(bIgnoreAllPressedKeysUntilRelease=True,bForceImmediately=False,bNotifyUserSettings=False)")
      (Input|AddMappingContext _returnvalue "/Game/Skvt/Characters/Input/IMC_SwapPawn.IMC_SwapPawn" 0 "(bIgnoreAllPressedKeysUntilRelease=True,bForceImmediately=False,bNotifyUserSettings=False)")
      (Input|AddMappingContext _returnvalue "/Game/Skvt/Characters/Input/IMC_Camera.IMC_Camera" 0 "(bIgnoreAllPressedKeysUntilRelease=True,bForceImmediately=False,bNotifyUserSettings=False)"))))

(fn ConstructionScript)

(fn IsMenuOpen
  (Utilities|IsValid (Variables|Default|GetMainMenuRef)
    (:Is%20Valid
      (return true))
    (:Is%20Not%20Valid
      (return false))))

(fn OpenMenu
  (bind _returnvalue (UserInterface|CreateWidget "/Game/Skvt/UI/Widgets/Menu/WBP_MainMenu.WBP_MainMenu_C" self))
  (bind _output_get (Variables|Default|SetMainMenuRef _returnvalue))
  (UserInterface|Viewport|AddtoViewport _output_get 0)
  (Variables|Default|SetbShowMouseCursor true)
  (Input|SetInputModeGameandUI self 0 "DoNotLock" true false)
  (Game|SetGamePaused true))

(fn CloseMenu
  (Utilities|IsValid (Variables|Default|GetMainMenuRef)
    (:Is%20Valid
      (Widget|RemovefromParent (Variables|Default|GetMainMenuRef))
      (Variables|Default|SetMainMenuRef 0)
      (Variables|Default|SetbShowMouseCursor false)
      (Input|SetInputModeGameOnly self false)
      (Game|SetGamePaused false))))

(fn FindNextChar
  (params (AvailableChar :type Array%20of%20Pawn%20Object%20References))
  (bind _returnvalue (Pawn|GetControlledPawn))
  (bind _returnvalue_2 (Utilities|Array|FindItem AvailableChar _returnvalue))
  (Utilities|FlowControl|Sequence
    (:then_0
      (if (Utilities|Array|IsValidIndex AvailableChar _returnvalue_2)
        (LocalVariables|SetCharIndex _returnvalue_2)
        (else
          (return 0))))
    (:then_1
      (if (Utilities|Array|IsValidIndex AvailableChar (+ (LocalVariables|GetCharIndex) 1))
        (return (Utilities|Array|Get(acopy) AvailableChar (+ (LocalVariables|GetCharIndex) 1)))
        (else
          (return (Utilities|Array|Get(acopy) AvailableChar)))))))