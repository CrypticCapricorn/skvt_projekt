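; BP_SkvtScreen is a screen actor that shows a WBP_SkvtWeb widget through its Webpage component and can be destroyed by an EMP.
; On BeginPlay it caches a reference to that widget.
; Toggleon sets the on state and the Webpage visibility unless the screen is already destroyed.
; DestroybyEMP spawns an explosion at the Webpage location, destroys the actor and sets the destroyed flag.
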(event EventBeginPlay
  (CallFunction|Initialize))

(event EventToggleon
  (params (IsItOn? :type Boolean))
  (if (not (Variables|Default|GetIsDestroyed?))
    (bind _output_get (Variables|Default|SetIsOn IsItOn?))
    (Rendering|SetVisibility (Variables|Default|GetWebpage) _output_get false)))

(event EventDestroybyEMP
  (CallFunction|DestroyObject))

(fn ConstructionScript)

(fn Initialize
  (bind _aswbp_skvt_web (Utilities|Casting|CastToWBP_SkvtWeb (UserInterface|GetWidget (Variables|Default|GetWebpage))))
  (Variables|Default|SetWebpageRef _aswbp_skvt_web))

(fn DestroyObject
  (Effects|SpawnEmitteratLocation "/Game/StarterContent/Particles/P_Explosion.P_Explosion" (Transformation|GetWorldLocation (Variables|Default|GetWebpage)))
  (Actor|DestroyActor)
  (Variables|Default|SetIsDestroyed? true)
  (return))